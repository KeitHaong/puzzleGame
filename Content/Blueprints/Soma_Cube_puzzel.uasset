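; Soma cube puzzle Blueprint that highlights mesh components with an outline material on overlap.
; The construction script adds a scaled static mesh and a larger box trigger at its location, then binds an event to begin overlap.
; One overlap handler replaces the other component's first material with a dynamic OutlineEffect instance.
; Its skeletal-mesh fallback leaves the created material unconnected, and two other generated handlers are empty.
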(fn ConstructionScript
  (bind _returnvalue (AddComponent|AddStaticMeshComponent false (Math|Transform|MakeTransform "0, 0, 0" "0, 0, 0" "1.500000,1.500000,1.500000")))
  (bind _returnvalue_2 (AddComponent|AddBoxComponent false (Math|Transform|MakeTransform (+ (Variables|/Script/Engine.SceneComponent|GetRelativeLocation _returnvalue) "") "0, 0, 0" "2.000000,2.000000,2.000000")))
  (Collision|BindEventtoOnComponentBeginOverlap _returnvalue_2 (EventDispatchers|CreateEvent :!event SomaCubePuzzelAutoGenFunc2)))

(fn SomaCubePuzzelAutoGenFunc
  (params (OverlappedComponent :type Primitive%20Component%20Object%20Reference) (OtherActor :type Actor%20Object%20Reference) (OtherComp :type Primitive%20Component%20Object%20Reference) (OtherBodyIndex :type Integer) (bFromSweep :type Boolean) (SweepResult :type Hit%20Result%20Structure%20%28by%20ref%29))
  (return))

(fn SomaCubePuzzelAutoGenFunc1
  (params (OverlappedComponent :type Primitive%20Component%20Object%20Reference) (OtherActor :type Actor%20Object%20Reference) (OtherComp :type Primitive%20Component%20Object%20Reference) (OtherBodyIndex :type Integer) (bFromSweep :type Boolean) (SweepResult :type Hit%20Result%20Structure%20%28by%20ref%29))
  (return))

(fn SomaCubePuzzelAutoGenFunc2
  (params (OverlappedComponent :type Primitive%20Component%20Object%20Reference) (OtherActor :type Actor%20Object%20Reference) (OtherComp :type Primitive%20Component%20Object%20Reference) (OtherBodyIndex :type Integer) (bFromSweep :type Boolean) (SweepResult :type Hit%20Result%20Structure%20%28by%20ref%29))
  (bind _asmesh_component (Utilities|Casting|CastToMeshComponent OtherComp)
    (:then
      (bind _returnvalue (Rendering|Material|CreateDynamicMaterialInstance "/Game/Blueprints/OutlineEffect.OutlineEffect" "None" "None" :!class /Script/Engine.KismetMaterialLibrary))
      (Rendering|Material|SetMaterial _asmesh_component 0 _returnvalue))
    (:CastFailed
      (bind _asskeletal_mesh_component (Utilities|Casting|CastToSkeletalMeshComponent OtherComp))
      (Rendering|Material|CreateDynamicMaterialInstance "/Game/Blueprints/OutlineEffect.OutlineEffect" "None" "None" :!class /Script/Engine.KismetMaterialLibrary)
      (Rendering|Material|SetMaterial _asskeletal_mesh_component 0 0))))