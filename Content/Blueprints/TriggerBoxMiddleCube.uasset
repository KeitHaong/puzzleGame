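; Trigger box actor that highlights its cube when a non-player actor overlaps it by enough volume.
; On begin overlap, CalculateOverLap computes the axis-aligned intersection volume of the trigger's bounds and the other actor's bounds.
; Above a fixed threshold the cube takes an outline material, otherwise the value prints for debugging.
; End overlap sets a transparent material, and BP_FirstPersonCharacter is ignored in both events.
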(event OnComponentBeginOverlap(BoxTrigger)
  (params (OverlappedComponent :type Primitive%20Component%20Object%20Reference) (OtherActor :type Actor%20Object%20Reference) (OtherComp :type Primitive%20Component%20Object%20Reference) (OtherBodyIndex :type Integer) (bFromSweep :type Boolean) (SweepResult :type Hit%20Result%20Structure%20%28by%20ref%29))
  (bind (_origin _boxextent) (Collision|GetActorBounds OtherActor false false))
  (bind _box_trigger (Variables|Default|GetBox%20Trigger))
  (bind (_origin_2 _boxextent_2) (Collision|GetComponentBounds _box_trigger))
  (Utilities|Casting|CastToBP_FirstPersonCharacter OtherActor
    (:CastFailed
      (if true
        (bind _overlapped_volume (CallFunction|CalculateOverLap (- _origin_2 _boxextent_2) (+ _origin_2 _boxextent_2) (- _origin _boxextent) (+ _origin _boxextent)))
        (if (> _overlapped_volume 5e+04)
          (Rendering|Material|SetMaterial (Variables|Default|GetCube) 0 "/Game/Blueprints/M_outline_cibe.M_outline_cibe")
          (else
            (Development|PrintString (Utilities|String|ToString(Float) _overlapped_volume) true true "(R=0.000000,G=0.660000,B=1.000000,A=1.000000)" 5.0 "Cant not get value")))))))

(event OnComponentEndOverlap(BoxTrigger)
  (params (OverlappedComponent :type Primitive%20Component%20Object%20Reference) (OtherActor :type Actor%20Object%20Reference) (OtherComp :type Primitive%20Component%20Object%20Reference) (OtherBodyIndex :type Integer))
  (Utilities|Casting|CastToBP_FirstPersonCharacter OtherActor
    (:CastFailed
      (if true
        (Rendering|Material|SetMaterial (Variables|Default|GetCube) 0 "/Game/Blueprints/FinalCubeTransparent.FinalCubeTransparent")))))

(fn ConstructionScript)

(fn CalculateOverLap
  (params (box1_min :type Vector) (box1_max :type Vector) (box2_min :type Vector) (box2_max :type Vector))
  (bind (_x _y _z) (Class|KismetMathLibrary|BreakVector3f box1_min))
  (bind (_x_2 _y_2 _z_2) (Class|KismetMathLibrary|BreakVector3f box1_max))
  (bind (_x_3 _y_3 _z_3) (Class|KismetMathLibrary|BreakVector3f box2_min))
  (bind (_x_4 _y_4 _z_4) (Class|KismetMathLibrary|BreakVector3f box2_max))
  (bind _returnvalue (Math|Float|Min(Float) _x_2 _x_4))
  (bind _returnvalue_2 (Math|Float|Min(Float) _y_2 _y_4))
  (bind _returnvalue_3 (Math|Float|Min(Float) _z_2 _z_4))
  (bind _returnvalue_4 (Math|Float|Max(Float) _x _x_3))
  (bind _returnvalue_5 (Math|Float|Max(Float) _y _y_3))
  (bind _returnvalue_6 (Math|Float|Max(Float) _z _z_3))
  (bind _returnvalue_7 (- _returnvalue _returnvalue_4))
  (bind _returnvalue_8 (- _returnvalue_2 _returnvalue_5))
  (bind _returnvalue_9 (- _returnvalue_3 _returnvalue_6))
  (bind _returnvalue_10 (Math|Float|Max(Float) _returnvalue_7 0.0))
  (bind _returnvalue_11 (Math|Float|Max(Float) _returnvalue_8 0.0))
  (bind _returnvalue_12 (Math|Float|Max(Float) _returnvalue_9 0.0))
  (bind _returnvalue_13 (* _returnvalue_10 _returnvalue_11))
  (bind _returnvalue_14 (* _returnvalue_13 _returnvalue_12))
  (Development|PrintString (Utilities|String|ToString(Float) _returnvalue_14))
  (return _returnvalue_14))